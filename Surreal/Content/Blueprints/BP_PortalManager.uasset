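; Portal manager that positions the scene captures of two portals and two windows each tick to follow the player camera.
; PortalUpdate offsets the camera location by the vector between Portal1 and Portal2, in opposite directions for each portal, and copies camera rotation to both.
; Both windows reuse Portal2's offset and are not fed the camera rotation.
; The offset is translation only, ignoring relative portal orientation.
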(event EventTick
  (params (DeltaSeconds :type Float%20%28single-precision%29))
  (CallFunction|PortalUpdate))

(fn ConstructionScript)

(fn PortalUpdate
  (bind _returnvalue (Game|GetPlayerCameraManager 0))
  (bind _transformcomponent (Variables|/Script/Engine.PlayerCameraManager|GetTransformComponent _returnvalue))
  (bind _returnvalue_2 (Transformation|GetWorldRotation _transformcomponent))
  (Transformation|SetWorldLocationAndRotation (Variables|/Game/Blueprints/BP_Portal2.BP_Portal2_C|GetPortalCapture (Variables|Default|GetPortal2)) (- (Transformation|GetWorldLocation (Variables|/Script/Engine.PlayerCameraManager|GetTransformComponent (Game|GetPlayerCameraManager 0))) (- (Transformation|GetWorldLocation (Variables|/Game/Blueprints/BP_Portal1.BP_Portal1_C|GetDefaultSceneRoot (Variables|Default|GetPortal1))) (Transformation|GetWorldLocation (Variables|/Game/Blueprints/BP_Portal2.BP_Portal2_C|GetDefaultSceneRoot (Variables|Default|GetPortal2))))) _returnvalue_2 false false)
  (Transformation|SetWorldLocationAndRotation (Variables|/Game/Blueprints/BP_Portal1.BP_Portal1_C|GetPortalCapture (Variables|Default|GetPortal1)) (- (Transformation|GetWorldLocation _transformcomponent) (- (Transformation|GetWorldLocation (Variables|/Game/Blueprints/BP_Portal2.BP_Portal2_C|GetDefaultSceneRoot (Variables|Default|GetPortal2))) (Transformation|GetWorldLocation (Variables|/Game/Blueprints/BP_Portal1.BP_Portal1_C|GetDefaultSceneRoot (Variables|Default|GetPortal1))))) _returnvalue_2 false false)
  (Transformation|SetWorldLocationAndRotation (Variables|/Game/Blueprints/Windows/BP_Window1Capture.BP_Window1Capture_C|GetPortalCapture (Variables|Default|GetWindow1)) (- (Transformation|GetWorldLocation (Variables|/Script/Engine.PlayerCameraManager|GetTransformComponent (Game|GetPlayerCameraManager 0))) (- (Transformation|GetWorldLocation (Variables|/Game/Blueprints/BP_Portal1.BP_Portal1_C|GetDefaultSceneRoot (Variables|Default|GetPortal1))) (Transformation|GetWorldLocation (Variables|/Game/Blueprints/BP_Portal2.BP_Portal2_C|GetDefaultSceneRoot (Variables|Default|GetPortal2))))) "0, 0, 0" false false)
  (Transformation|SetWorldLocationAndRotation (Variables|/Game/Blueprints/Windows/BP_Window2Capture.BP_Window2Capture_C|GetPortalCapture (Variables|Default|GetWindow2)) (- (Transformation|GetWorldLocation (Variables|/Script/Engine.PlayerCameraManager|GetTransformComponent (Game|GetPlayerCameraManager 0))) (- (Transformation|GetWorldLocation (Variables|/Game/Blueprints/BP_Portal1.BP_Portal1_C|GetDefaultSceneRoot (Variables|Default|GetPortal1))) (Transformation|GetWorldLocation (Variables|/Game/Blueprints/BP_Portal2.BP_Portal2_C|GetDefaultSceneRoot (Variables|Default|GetPortal2))))) "0, 0, 0" false false))