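; CanReadLetter is an interactable letter actor that the player can read by pressing E while nearby.
; Overlapping its Box enables input and opens a Gate, letting E toggle IsReading.
; Reading hides the Paper component and shows a newly created ReadLetterWidget; closing restores the paper and removes the widget.
; Leaving the Box disables input and runs the same closing path, without closing the Gate.
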(event OnComponentBeginOverlap(Box)
  (params (OtherActor :type Actor%20Object%20Reference) (OtherComp :type Primitive%20Component%20Object%20Reference) (OtherBodyIndex :type Integer) (bFromSweep :type Boolean) (SweepResult :type Hit%20Result%20Structure%20%28by%20ref%29))
  (bind _paper (Variables|Default|GetPaper))
  (Input|EnableInput (Game|GetPlayerController 0))
  (Utilities|FlowControl|Gate true) ; enters at Open
)

(event OnComponentEndOverlap(Box)
  (params (OtherActor :type Actor%20Object%20Reference) (OtherComp :type Primitive%20Component%20Object%20Reference) (OtherBodyIndex :type Integer))
  (Input|DisableInput (Game|GetPlayerController 0))
  (Variables|Default|SetisReading false)
  (Development|SetHiddeninGame (Variables|Default|GetPaper) false false)
  (Widget|RemovefromParent (stale Input|KeyboardEvents|E _returnvalue)))

(event EventBeginPlay)

(event EventActorBeginOverlap
  (params (OtherActor :type Actor%20Object%20Reference)))

(event EventTick
  (params (DeltaSeconds :type Float%20%28single-precision%29)))

(event Input|KeyboardEvents|E
  (params (Key :type Key%20Structure :default "AnyKey"))
  (bind _paper (Variables|Default|GetPaper))
  (:Pressed
    (Utilities|FlowControl|Gate true
      (:Exit
        (if (Variables|Default|GetisReading)
          (Variables|Default|SetisReading false)
          (Development|SetHiddeninGame _paper false false)
          (Widget|RemovefromParent (stale _returnvalue))
          (else
            (Variables|Default|SetisReading true)
            (Development|SetHiddeninGame _paper true false)
            (bind _returnvalue (UserInterface|CreateWidget "/Game/Textures/ReadLetterWidget.ReadLetterWidget_C"))
            (UserInterface|Viewport|AddtoViewport _returnvalue 0)))))))

(fn ConstructionScript)